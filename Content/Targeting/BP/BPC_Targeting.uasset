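; Lock-on targeting component for a Character owner that stores a chosen actor as LockedTarget.
; LockonTarget gathers BPI_Target actors with a sphere trace around the character, then picks among those whose camera-to-target visibility trace hits something.
; The highest dot product of target-to-camera direction and normalized camera world position wins, rather than using camera facing.
; Candidates and best score persist between calls, and debug traces and prints remain enabled.
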(event `self.ReceiveBeginPlay`
  (bind _ascharacter (cast `Character` (`self.GetOwner`)))
  (set `self.Character Ref` _ascharacter)
  (set `self.Camera Ref` (`Actor.GetComponentByClass` (`self.Character Ref`) "/Script/Engine.CameraComponent")))

(event `Lock on Target`
  (bind _closest_target (`self.Get Closest Target` (`self.Find Potential Targets`)))
  (`/Engine/EditorBlueprintResources/StandardMacros.IsValid` _closest_target
    (:`Is Valid`
      (set `self.Locked Target` _closest_target))))

(fn `Check How Close Target`
  (params (Target :type "Actor Object Reference"))
  (returns (`dot product` :type "Float (double-precision)"))
  (locals (`Dir To Enemy Normalized` :type "Vector Structure"))
  (bind _returnvalue (`SceneComponent.K2_GetComponentLocation` (`self.Camera Ref`)))
  (bind _output_get (set `local.Dir To Enemy Normalized` (`KismetMathLibrary.Normal` (- _returnvalue (`Actor.K2_GetActorLocation` Target)))))
  (return (`KismetMathLibrary.Dot_VectorVector` _output_get (`KismetMathLibrary.Normal` (`KismetMathLibrary.GetForwardVector` (`KismetMathLibrary.Conv_VectorToRotator` _returnvalue))))))

(fn `Find Potential Targets`
  (returns (`Potential Targets` :type "Array of Actor Object Reference"))
  (locals (Radius :type "Float (double-precision)" :default 500.0) (`Poteintal Targets` :type "Array of Actor Object Reference"))
  (bind _character_ref (`self.Character Ref`))
  (bind _returnvalue (`Actor.K2_GetActorLocation` _character_ref))
  (bind (_outhits _returnvalue_2) (`KismetSystemLibrary.SphereTraceMultiForObjects` _returnvalue _returnvalue (`local.Radius`) (`|MakeArray` "ObjectTypeQuery7" :!type "EObjectTypeQuery Enum") false (`|MakeArray` _character_ref) "ForDuration"))
  (for _array_element _outhits
    (bind (_bblockinghit _binitialoverlap _time _distance _location _impactpoint _normal _impactnormal _physmat _hitactor) (`GameplayStatics.BreakHitResult` _array_element))
    (if (and (`KismetSystemLibrary.DoesImplementInterface` _hitactor "/Game/Targeting/BP/BPI_Target.BPI_Target_C") _returnvalue_2)
      (`KismetArrayLibrary.Array_Add` (`local.Poteintal Targets`) _hitactor)))
  (return (`local.Poteintal Targets`)))

(fn `Get Closest Target`
  (params (`Potential Targets` :type "Array of Actor Object Reference"))
  (returns (`Closest Target` :type "Actor Object Reference"))
  (locals (`Closest Target Normal` :type "Float (double-precision)" :default -1.0) (`Closest Target Actor` :type "Actor Object Reference"))
  (for _array_element `Potential Targets`
    (bind (_outhit _returnvalue) (`KismetSystemLibrary.LineTraceSingle` :`Start` (`SceneComponent.K2_GetComponentLocation` (`self.Camera Ref`)) :`End` (`Actor.K2_GetActorLocation` _array_element) :`TraceChannel` "TraceTypeQuery1" :`DrawDebugType` "ForDuration"))
    (if _returnvalue
      (bind _dot_product (`self.Check How Close Target` _array_element))
      (`KismetSystemLibrary.PrintString` (`KismetStringLibrary.Concat_StrStr` (`KismetSystemLibrary.GetDisplayName` _array_element) " " (`KismetStringLibrary.Conv_DoubleToString` _dot_product)))
      (`/Engine/EditorBlueprintResources/StandardMacros.CompareFloat` _dot_product (`local.Closest Target Normal`)
        (:`>`
          (set `local.Closest Target Normal` _dot_product)
          (set `local.Closest Target Actor` _array_element)))))
  (return (`local.Closest Target Actor`)))